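; Grippable pétanque ball for VR characters, thrown with a charged force.
; Gripping enables input and shows a throw-bar widget to the local player; holding use runs a timeline that raises the force.
; Ending use drops the ball and applies an impulse along the replicated camera's forward vector.
; Charge and throw run locally and relay through server-to-multicast events; secondary use is an empty stub with disconnected dribble logic.
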(event Custom|ChargeServer
  ;[1 1 1] Charge the event on the server and will call the multicast event to replicate it to all client
  (CallFunction|ChargeMulticast))

(event Custom|ChargeMulticast
  ;[1 1 1] Charge event multicast, will replicate the local event on all client
  (bind _ascharacter (Utilities|Casting|CastToCharacter (Components|GetOwner)))
  (if (not (Pawn|IsLocallyControlled _ascharacter))
    (CallFunction|ChargeLocal)))

(event Custom|ChargeLocal
  ;[1 1 1] Charge the force amount it has to be throw
  (bind _chargecurve (Timeline|ChargeTimeline PlayFromStart) ; Timeline, it's a loop that can be modified when double clicked
    (:Update
      (Variables|Default|SetThrowForce (Math|Float|Lerp (Math|Random|RandomFloatinRange 2e+01 8e+01) (Variables|Default|GetMaxThrowForce) _chargecurve)))))

(event Custom|ThrowMulticast
  ;[1 1 1] Throw event
  ;;[1 1 1] Multicast play the local event, so it replicates it to everyone
  (CallFunction|ThrowLocal))

(event Custom|ThrowServer
  ;[1 1 1] Throw event
  ;;[1 1 1] Triggered from local, now calls it on the server and replicate it to all client (grâce à multicast)
  (CallFunction|ThrowMulticast))

(event Custom|Remove%20widget
  ;[1 1 1] Remove/Add widget event - Throw force progress widget
  (bind _wb_throwbar (Variables|Default|GetWB_ThrowBar)
    (:then
      (Widget|RemovefromParent _wb_throwbar))
    (:else)))

(event Custom|Add%20widget
  ;[1 1 1] Remove/Add widget event - Throw force progress widget
  (bind _returnvalue (UserInterface|CreateWidget "/Game/VRE/Basketball/WB_ThrowBar.WB_ThrowBar_C" 0 self (Variables|Default|GetMaxThrowForce)))
  (bind _output_get (Variables|Default|SetWB_ThrowBar _returnvalue))
  (UserInterface|Viewport|AddtoViewport _output_get 0))

(event Custom|ThrowLocal
  (bind _staticmeshcomponent (Variables|Default|GetStaticMeshComponent))
  ;[1 1 1] Throw event
  (Utilities|FlowControl|Sequence ; Sequence, first do 0 then 1 then more...
    (:then_0
      ;[1 1 1] Charge the force amount it has to be throw
      (bind _chargecurve (Timeline|ChargeTimeline Stop) ; Timeline, it's a loop that can be modified when double clicked
        (:Update
          (Variables|Default|SetThrowForce (Math|Float|Lerp (Math|Random|RandomFloatinRange 2e+01 8e+01) (Variables|Default|GetMaxThrowForce) _chargecurve)))))
    (:then_1
      (Class|GripMotionControllerComponent|DropObject (Variables|Default|GetGripping%20Controller) self 0 false "0, 0, 0" "0, 0, 0") ; We then drop the object
      (bind _asfps_vrcharacter (Utilities|Casting|CastToFPS_VRCharacter (Components|GetOwner))) ; Get the FPS Vr character
      (Physics|SetSimulatePhysics _staticmeshcomponent true) ; Simulate the physics
      (Physics|AddImpulse _staticmeshcomponent (* (Math|Vector|GetForwardVector (Variables|/Script/VRExpansionPlugin.VRBaseCharacter|GetVRReplicatedCamera _asfps_vrcharacter)) (Variables|Default|GetThrowForce)) "None" false) ; Add an impulse based on the \nplayer charge (throw force)
      ;;[1 0.7253 0.1605] Reset some variables and disable the input (so the player cant use the bp event tho he doesnt have it)
      (Input|DisableInput (Game|GetPlayerController 0))
      (Variables|Default|SetThrowForce 0.0)
      (Variables|Default|Setgrabbed? false)
      (CallFunction|RemoveWidget) ; Remove the throw force widget from the player's screen
    )))

(event EventOnGrip
  (params (GrippingController :type Grip%20Motion%20Controller%20Component%20Object%20Reference) (GripInformation :type BP%20Actor%20Grip%20Information%20Structure%20%28by%20ref%29))
  ;[1 1 1] Player grabbed the object
  (Variables|Default|SetGripping%20Controller GrippingController)
  (Input|EnableInput (Game|GetPlayerController 0))
  (bind _asfps_vrcharacter (Utilities|Casting|CastToFPS_VRCharacter (Components|GetOwner) :!label _label)
    (:then
      (GameplayTags|AddGameplayTag (Variables|Default|GetGameplayTags) "(TagName=\"DropType.OnAltGrip\")" :!class /Script/GameplayTags.BlueprintGameplayTagLibrary)
      (if (Pawn|IsLocallyControlled _asfps_vrcharacter)
        (CallFunction|AddWidget)
        (Utilities|FlowControl|Delay 0.2)
        (Variables|Default|Setgrabbed? true)))
    (:CastFailed
      (Utilities|FlowControl|Delay 0.2) ; in case the cast failed on first grip
      (goto _label))))

(event EventOnSecondaryUsed
  ;[1 1 1] Secondary use event, maybe for another feature or has to be removed later
)

(event EventOnUsed
  ;[1 1 1] Event used triggered, will now call the charge event server and local
  (CallFunction|ChargeServer)
  (CallFunction|ChargeLocal)
  (Variables|Default|Setgrabbed? false))

(event EventOnGripRelease
  (params (ReleasingController :type Grip%20Motion%20Controller%20Component%20Object%20Reference) (GripInformation :type BP%20Actor%20Grip%20Information%20Structure%20%28by%20ref%29) (bWasSocketed :type Boolean))
  ;[1 1 1] Player grabbed the object
  ;;[1 1 1] Player dropped the object
  (bind _bisheld (Class|VRGripInterface|IsHeld))
  (if _bisheld
    (Physics|AddImpulse (Variables|Default|GetStaticMeshComponent) (* (Transformation|GetComponentVelocity (Variables|Default|GetGripping%20Controller)) 2e+02) "None" false)
    (Variables|Default|SetGripping%20Controller 0)
    (else
      (Input|DisableInput (Game|GetPlayerController 0)))))

(event EventOnEndUsed
  ;[1 1 1] Throw event
  ;;[1 1 1] Event triggered
  (CallFunction|ThrowServer)
  (CallFunction|ThrowLocal))

(fn ConstructionScript)