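; Basketball hoop actor for the VR game that detects baskets and shows the score on a text render.
; Three trigger volumes above, in the middle and below set server-side flags when a BP_Basketball overlaps them.
; The below trigger runs the scoring check, adding a point if all three flags are set, then clearing them.
; A below-only hit counts as cheating and pauses detection briefly.
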(event OnComponentBeginOverlap(CollisionCheckMiddle)
  (params (OverlappedComponent :type Primitive%20Component%20Object%20Reference) (OtherActor :type Actor%20Object%20Reference) (OtherComp :type Primitive%20Component%20Object%20Reference) (OtherBodyIndex :type Integer) (bFromSweep :type Boolean) (SweepResult :type Hit%20Result%20Structure%20%28by%20ref%29))
  (if (not (Variables|Default|GetCheatTimer))
    (Utilities|Casting|CastToBP_Basketball OtherActor)
    (Networking|SwitchHasAuthority
      (:Authority
        (Variables|Default|SetMiddleOverlapped? true)))))

(event OnComponentBeginOverlap(CollisionCheckAbove)
  (params (OverlappedComponent :type Primitive%20Component%20Object%20Reference) (OtherActor :type Actor%20Object%20Reference) (OtherComp :type Primitive%20Component%20Object%20Reference) (OtherBodyIndex :type Integer) (bFromSweep :type Boolean) (SweepResult :type Hit%20Result%20Structure%20%28by%20ref%29))
  (if (not (Variables|Default|GetCheatTimer))
    (Utilities|Casting|CastToBP_Basketball OtherActor)
    (Networking|SwitchHasAuthority
      (:Authority
        (Variables|Default|SetAboveOverlapped? true)))))

(event OnComponentBeginOverlap(CollisionCheckBelow)
  (params (OverlappedComponent :type Primitive%20Component%20Object%20Reference) (OtherActor :type Actor%20Object%20Reference) (OtherComp :type Primitive%20Component%20Object%20Reference) (OtherBodyIndex :type Integer) (bFromSweep :type Boolean) (SweepResult :type Hit%20Result%20Structure%20%28by%20ref%29))
  (if (not (Variables|Default|GetCheatTimer))
    (Utilities|Casting|CastToBP_Basketball OtherActor)
    (Networking|SwitchHasAuthority
      (:Authority
        (Variables|Default|SetBelowOverlapped? true)
        (CallFunction|ScoringCheck)))))

(event Custom|ScoringCheck
  (Development|PrintString "check if goal is correct")
  (if (Math|Boolean|ANDBoolean (Variables|Default|GetBelowOverlapped?) (not (Variables|Default|GetAboveOverlapped?)) (not (Variables|Default|GetMiddleOverlapped?))) ; anticheat
    (Variables|Default|SetAboveOverlapped? false)
    (Variables|Default|SetBelowOverlapped? false)
    (Variables|Default|SetMiddleOverlapped? false)
    (Development|PrintString "caught cheating")
    (Variables|Default|SetCheatTimer true)
    (Utilities|FlowControl|Delay 2.0)
    (Variables|Default|SetCheatTimer false)
    (elif (Math|Boolean|ANDBoolean (Variables|Default|GetAboveOverlapped?) (Variables|Default|GetMiddleOverlapped?) (Variables|Default|GetBelowOverlapped?))
      (Development|PrintString "SCORE GOOD!!")
      (Variables|Default|SetAboveOverlapped? false)
      (Variables|Default|SetBelowOverlapped? false)
      (Variables|Default|SetMiddleOverlapped? false)
      (Variables|Default|SetScore (+ (Variables|Default|GetScore) 1))
      (CallFunction|UpdateScoreText)
      (else
        (Development|PrintString "didnt score..")
        (Variables|Default|SetAboveOverlapped? false)
        (Variables|Default|SetBelowOverlapped? false)
        (Variables|Default|SetMiddleOverlapped? false)))))

(event Custom|UpdateScoreText
  (CallFunction|SetScoreText))

(fn ConstructionScript)

(fn SetScoreText
  (Rendering|Components|TextRender|SetText (Variables|Default|GetTextRender) (Utilities|Text|ToText(Integer) (Variables|Default|GetScore))))