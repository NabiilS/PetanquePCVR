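; Grippable VR basketball that the holder can dribble, or throw with a charged shot.
; Gripping enables input and shows a throw-bar widget to the local player; secondary use drops the ball with a slightly randomized dribble impulse.
; Use runs a timeline that raises throw force; ending use launches along the camera's forward vector.
; Charge and throw run locally and relay through server-to-multicast events, with only charge skipping the locally controlled owner.
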(event Custom|ChargeServer
  (CallFunction|ChargeMulticast))

(event Custom|ChargeMulticast
  (bind _ascharacter (Utilities|Casting|CastToCharacter (Components|GetOwner)))
  (if (not (Pawn|IsLocallyControlled _ascharacter))
    (CallFunction|ChargeLocal)))

(event Custom|ChargeLocal
  (bind _chargecurve (Timeline|ChargeTimeline PlayFromStart)
    (:Update
      (Variables|Default|SetThrowForce (Math|Float|Lerp (Math|Random|RandomFloatinRange 2e+01 8e+01) (Variables|Default|GetMaxThrowForce) _chargecurve)))))

(event Custom|ThrowMulticast
  (CallFunction|ThrowLocal))

(event Custom|ThrowServer
  (CallFunction|ThrowMulticast))

(event Custom|Remove%20widget
  (bind _wb_throwbar (Variables|Default|GetWB_ThrowBar)
    (:then
      (Widget|RemovefromParent _wb_throwbar))
    (:else)))

(event Custom|Add%20widget
  (bind _returnvalue (UserInterface|CreateWidget "/Game/VRE/Basketball/WB_ThrowBar.WB_ThrowBar_C" 0 self (Variables|Default|GetMaxThrowForce)))
  (bind _output_get (Variables|Default|SetWB_ThrowBar _returnvalue))
  (UserInterface|Viewport|AddtoViewport _output_get 0))

(event Custom|ThrowLocal
  (bind _staticmeshcomponent (Variables|Default|GetStaticMeshComponent))
  (Utilities|FlowControl|Sequence
    (:then_0
      (bind _chargecurve (Timeline|ChargeTimeline Stop)
        (:Update
          (Variables|Default|SetThrowForce (Math|Float|Lerp (Math|Random|RandomFloatinRange 2e+01 8e+01) (Variables|Default|GetMaxThrowForce) _chargecurve)))))
    (:then_1
      (Class|GripMotionControllerComponent|DropObject (Variables|Default|GetGripping%20Controller) self 0 false "0, 0, 0" "0, 0, 0")
      (bind _asfps_vrcharacter (Utilities|Casting|CastToFPS_VRCharacter (Components|GetOwner)))
      (Physics|SetSimulatePhysics _staticmeshcomponent true)
      (Physics|AddImpulse _staticmeshcomponent (* (Math|Vector|GetForwardVector (Variables|/Script/VRExpansionPlugin.VRBaseCharacter|GetVRReplicatedCamera _asfps_vrcharacter)) (Variables|Default|GetThrowForce)) "None" false)
      (Input|DisableInput (Game|GetPlayerController 0))
      (Variables|Default|SetThrowForce 0.0)
      (Variables|Default|Setgrabbed? false)
      (CallFunction|RemoveWidget))))

(event EventOnGrip
  (params (GrippingController :type Grip%20Motion%20Controller%20Component%20Object%20Reference) (GripInformation :type BP%20Actor%20Grip%20Information%20Structure%20%28by%20ref%29))
  (Variables|Default|SetGripping%20Controller GrippingController)
  (Input|EnableInput (Game|GetPlayerController 0))
  (bind _asfps_vrcharacter (Utilities|Casting|CastToFPS_VRCharacter (Components|GetOwner) :!label _label)
    (:then
      (GameplayTags|AddGameplayTag (Variables|Default|GetGameplayTags) "(TagName=\"DropType.OnAltGrip\")" :!class /Script/GameplayTags.BlueprintGameplayTagLibrary)
      (if (Pawn|IsLocallyControlled _asfps_vrcharacter)
        (CallFunction|AddWidget)
        (Utilities|FlowControl|Delay 0.2)
        (Variables|Default|Setgrabbed? true)))
    (:CastFailed
      (Development|PrintString "cast failed")
      (Utilities|FlowControl|Delay 0.2)
      (goto _label))))

(event EventOnSecondaryUsed
  (bind _staticmeshcomponent (Variables|Default|GetStaticMeshComponent))
  (if (Variables|Default|Getgrabbed?)
    (Development|PrintString "secondary use")
    (bind _asfps_vrcharacter (Utilities|Casting|CastToFPS_VRCharacter (Components|GetOwner)))
    (Class|GripMotionControllerComponent|DropObject (Variables|Default|GetGripping%20Controller) self 0 false "0, 0, 0" "0, 0, 0")
    (Development|PrintString (Utilities|String|ToString(Vector) (Math|Conversions|ToVector(Float) (.x (Transformation|GetVelocity _asfps_vrcharacter)))))
    (Physics|SetSimulatePhysics _staticmeshcomponent true)
    (Physics|AddImpulse _staticmeshcomponent (* (Math|Vector|MakeVector (Math|Random|RandomFloatinRange 0.1 0.4) 0.0 1.3) (Variables|Default|GetDribbleForce)) "None" false)
    (Input|DisableInput (Game|GetPlayerController 0))
    (Variables|Default|SetThrowForce 0.0)
    (Variables|Default|Setgrabbed? false)
    (CallFunction|RemoveWidget)))

(event EventOnUsed
  (CallFunction|ChargeServer)
  (CallFunction|ChargeLocal)
  (Variables|Default|Setgrabbed? false))

(event EventOnGripRelease
  (params (ReleasingController :type Grip%20Motion%20Controller%20Component%20Object%20Reference) (GripInformation :type BP%20Actor%20Grip%20Information%20Structure%20%28by%20ref%29) (bWasSocketed :type Boolean))
  (bind _bisheld (Class|VRGripInterface|IsHeld))
  (if _bisheld
    (Physics|AddImpulse (Variables|Default|GetStaticMeshComponent) (* (Transformation|GetComponentVelocity (Variables|Default|GetGripping%20Controller)) 2e+02) "None" false)
    (Variables|Default|SetGripping%20Controller 0)
    (else
      (Input|DisableInput (Game|GetPlayerController 0)))))

(event EventOnEndUsed
  (CallFunction|ThrowServer)
  (CallFunction|ThrowLocal))

(fn ConstructionScript)